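; NPC character that shoots at the player and tracks its own Health when damaged.
; ShootAttack plays the firing effects, then line-traces on Visibility from the NPC to the player, applying fixed damage if the hit actor passes an equality check.
; PlayShootFX plays a montage on the mesh, then spawns an emitter at the gun mesh.
; AnyDamage sets Health to Damage minus Health, the reverse of a usual subtraction.
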(event `self.ReceiveAnyDamage`
  (params (Damage :type "Float (single-precision)") (DamageType :type "DamageType Object Reference") (InstigatedBy :type "Controller Object Reference") (DamageCauser :type "Actor Object Reference"))
  ;[1 1 1] Damage applied to Health
  (set `self.Health` (- Damage (`self.Health`)))
  (`KismetSystemLibrary.PrintString` "Receiving damage"))

(event `\`Shoot Attack`
  ;[1 1 1] Raycast to target Player
  (`self.Play ShootFX`)
  (bind (_outhit _returnvalue) (`KismetSystemLibrary.LineTraceSingle` :`Start` (`self.K2_GetActorLocation`) :`End` (`self.K2_GetActorLocation` (`GameplayStatics.GetPlayerCharacter` 0)) :`TraceChannel` "TraceTypeQuery1" :`DrawDebugType` "ForDuration"))
  (if _returnvalue
    (bind (_bblockinghit _binitialoverlap _time _distance _location _impactpoint _normal _impactnormal _physmat _hitactor) (`GameplayStatics.BreakHitResult` _outhit))
    (if (== _hitactor null)
      (`GameplayStatics.ApplyDamage` _hitactor 20.0 (`self.GetController`) self "/Script/Engine.DamageType")
      (`KismetSystemLibrary.PrintString` "Damage applied"))))

(event `Play ShootFX`
  (bind _gunmesh (`self.GunMesh`))
  ;[1 1 1] Shoot Animation and Effects
  (`|PlayMontage` (`self.Mesh`)
    (:`then`
      (`GameplayStatics.SpawnEmitterAtLocation` null (`SceneComponent.GetSocketLocation` _gunmesh "None") (`SceneComponent.GetSocketRotation` _gunmesh "None") (1.0 1.0 1.0) true "AutoRelease"))))

(fn `UserConstructionScript`)